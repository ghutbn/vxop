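; BP_MoveRect is a test actor that moves its StaticMesh around a square path in the local X-Z plane.
; BeginPlay starts a looping timer that calls UpdateMove, which steps the mesh in the MoveType direction and switches to the next direction past each bound.
; R press and release only print debug text.
; Unconnected leftovers hold a left-right ping-pong variant, delayed timer clearing and input toggling.
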(event `Key|R`
  (params (Key :type "Key Structure"))
  (:`Pressed`
    (`KismetSystemLibrary.PrintString` "1"))
  (:`Released`
    (`KismetSystemLibrary.PrintString` "0")))

(event `self.ReceiveBeginPlay`
  (`KismetSystemLibrary.K2_SetTimer` null "UpdateMove" 0.01 true))

(fn `UpdateMove`
  (bind _staticmesh (`self.StaticMesh`))
  (bind _relativelocation_x (`KismetMathLibrary.BreakVector` (`SceneComponent.RelativeLocation` (`self.StaticMesh`))))
  (bind (_relativelocation_x_2 _relativelocation_y _relativelocation_z) (`KismetMathLibrary.BreakVector` (`SceneComponent.RelativeLocation` (`self.StaticMesh`))))
  (bind _relativelocation_x_3 (`KismetMathLibrary.BreakVector` (`SceneComponent.RelativeLocation` (`self.StaticMesh`))))
  (bind (_relativelocation_x_4 _relativelocation_y_2 _relativelocation_z_2) (`KismetMathLibrary.BreakVector` (`SceneComponent.RelativeLocation` (`self.StaticMesh`))))
  ;[1 1 1] RightLeftUpDown
  (switch `/Game/helloUnreal/EN_MoveType` (`self.MoveType`)
    (:`NewEnumerator0`
      (`SceneComponent.K2_AddRelativeLocation` _staticmesh (10.0 0.0 0.0) false false)
      (if (> _relativelocation_x 1000.0)
        (set `self.MoveType` "NewEnumerator1")))
    (:`NewEnumerator1`
      (`SceneComponent.K2_AddRelativeLocation` _staticmesh (0.0 0.0 10.0) false false)
      (if (> _relativelocation_z 1000.0)
        (set `self.MoveType` "NewEnumerator2")))
    (:`NewEnumerator2`
      (`SceneComponent.K2_AddRelativeLocation` _staticmesh (-10.0 0.0 0.0) false false)
      (if (> 0.0 _relativelocation_x_3)
        (set `self.MoveType` "NewEnumerator3")))
    (:`NewEnumerator3`
      (`SceneComponent.K2_AddRelativeLocation` _staticmesh (0.0 0.0 -10.0) false false)
      (if (> 0.0 _relativelocation_z_2)
        (set `self.MoveType` "NewEnumerator0")))))

(fn `UserConstructionScript`)