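; BP_MyBox is a trigger box that starts other moving objects when something overlaps its Cube2 component.
; On overlap it prints the names of the components and actor involved, then calls Play on every element of the MoveRect, RotationBall and LeftRight arrays in sequence.
; Unconnected loop and Sequence nodes that print number ranges remain in the graph and never run.
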(event `self.ReceiveBeginPlay`)

(event `self.Cube2.OnComponentBeginOverlap`
  (params (OverlappedComponent :type "PrimitiveComponent Object Reference") (OtherActor :type "Actor Object Reference") (OtherComp :type "PrimitiveComponent Object Reference") (OtherBodyIndex :type Integer) (bFromSweep :type Boolean) (SweepResult :type "HitResult Structure (by ref)"))
  (`KismetSystemLibrary.PrintString` (`KismetStringLibrary.Concat_StrStr` " a: " (`KismetSystemLibrary.GetDisplayName` OverlappedComponent) " b: " (`KismetSystemLibrary.GetDisplayName` OtherActor) " c: " (`KismetSystemLibrary.GetDisplayName` OtherComp)))
  (`|ExecutionSequence`
    (:`then_0`
      (for _array_element (`self.MoveRect`)
        (`/Game/HelloUnreal/BP_MoveRect.Play` _array_element)))
    (:`then_1`
      (for _array_element_2 (`self.RotationBall`)
        (`/Game/HelloUnreal/BP_RotationBall.Play` _array_element_2)))
    (:`then_2`
      (for _array_element_3 (`self.LeftRight`)
        (`/Game/HelloUnreal/BP_MoveLeftRight.Play` _array_element_3)))))

(fn `UserConstructionScript`)